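; HexGridBP is an actor that builds a hexagon-shaped grid of tile meshes in its Construction Script.
; It derives tile size from the TileMesh bounds plus Margin, then loops over axial coordinates, keeping cells with distance below Radius.
; AddTile converts each coordinate to a position and adds a static mesh component.
; An IsAxis check via cube coordinates exists, but its result is unused.
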(fn `AddTile`
  (params (map_X :type Integer) (map_Y :type Integer))
  (`self.IsAxis` map_X map_Y)
  (bind _returnvalue (`GKHexGridUtilities.GridToWorld` (`self.TileSize`) (make `IntVector` map_X map_Y)))
  (if false
    (`AddComponent|NODE_AddStaticMeshComponent-2` :`RelativeTransform` (`KismetMathLibrary.MakeTransform` _returnvalue))
    (else
      (`AddComponent|NODE_AddStaticMeshComponent-0` :`RelativeTransform` (`KismetMathLibrary.MakeTransform` _returnvalue)))))

(fn `IsAxis`
  (params (X :type Integer) (Y :type Integer))
  (returns (IsAxis :type Boolean))
  (bind _returnvalue (`GKHexGridUtilities.AxialToCube` (`KismetMathLibrary.MakeVector2D` (`KismetMathLibrary.Conv_IntToDouble` X) (`KismetMathLibrary.Conv_IntToDouble` Y))))
  (return (or (== (`KismetMathLibrary.FTrunc` (.x _returnvalue)) 0) (== (`KismetMathLibrary.FTrunc` (.y _returnvalue)) 0) (== 0 (`KismetMathLibrary.FTrunc` (.z _returnvalue))))))

(fn `Set Tile Size`
  (returns (NewParam :type "Vector2D Structure"))
  (locals (TileMesh :type "StaticMesh Object Reference" :default "StaticMesh'/Game/Tile/HexMesh.HexMesh'"))
  (bind (_min _max) (break `Box` (`StaticMesh.GetBoundingBox` (`local.TileMesh`))))
  (bind _returnvalue (`GKHexGridUtilities.GetHexSize` (+ (- _max _min) (`self.Margin`))))
  (bind _output_get (set `self.TileSize` _returnvalue))
  (return _output_get))

(fn `UserConstructionScript`
  (locals (X :type Integer :default 5) (Y :type Integer :default 5) (HexMesh :type "StaticMesh Object Reference" :default "StaticMesh'/Game/Tile/HexMesh.HexMesh'"))
  (bind _radius (`self.Radius`))
  (bind _returnvalue (* _radius -1))
  (`self.Set Tile Size`)
  (for _index (range _returnvalue (+ _radius 1))
    (for _index_2 (range _returnvalue (+ _radius 1))
      (bind _returnvalue_2 (`GKHexGridUtilities.Distance` (make `IntPoint` _index_2 _index) (make `IntPoint` 0)))
      (if (< _returnvalue_2 (`KismetMathLibrary.Conv_IntToDouble` (`self.Radius`)))
        (`self.AddTile` _index_2 _index)))))