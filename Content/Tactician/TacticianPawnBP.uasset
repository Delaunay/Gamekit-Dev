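; TacticianPawnBP is the player pawn for the tactician view, providing middle-mouse drag panning.
; Pressing the middle mouse button records the cursor position and sets a grab flag; releasing clears it.
; While grabbing, Tick converts the per-frame cursor delta, scaled by CameraGrabSensitivity, into a world-space X/Y offset of the pawn, with screen axes swapped and horizontal movement inverted.
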(event `self.ReceiveTick`
  (params (DeltaSeconds :type "Float (single-precision)"))
  (bind (_mouseposstart_x _mouseposstart_y) (`KismetMathLibrary.BreakVector2D` (`self.MousePosStart`)))
  (bind (_locationx _locationy) (`PlayerController.GetMousePosition` (`GameplayStatics.GetPlayerController` 0)))
  (if (`self.CameraGrab`)
    (`self.K2_AddActorWorldOffset` (`KismetMathLibrary.MakeVector` (* (- _locationy _mouseposstart_y) (`self.CameraGrabSensitivity`)) (* (- _mouseposstart_x _locationx) (`self.CameraGrabSensitivity`))))
    (set `self.MousePosStart` (`KismetMathLibrary.MakeVector2D` _locationx _locationy))))

(event `Key|MiddleMouseButton`
  (params (Key :type "Key Structure"))
  (bind (_locationx _locationy) (`PlayerController.GetMousePosition` (`GameplayStatics.GetPlayerController` 0)))
  (:`Pressed`
    (set `self.MousePosStart` (`KismetMathLibrary.MakeVector2D` _locationx _locationy))
    (set `self.CameraGrab` true))
  (:`Released`
    (set `self.CameraGrab` false)))

(fn `UserConstructionScript`)