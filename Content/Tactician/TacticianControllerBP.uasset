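; Tactician controller Blueprint that updates the HUD and tile range highlight when units are selected or unselected.
; Selection shows the unit's preview in the HUD's main widget and writes its mesh location and a fixed range to the TileMatParameters material parameter collection, which drives the range display.
; Unselection removes the preview and hides the range, reusing the HUD cast from selection.
; BeginPlay only prints a ready message; the CollisionMapDrawer spawning logic is disconnected.
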(event `self.ReceiveBeginPlay`
  (`KismetSystemLibrary.PrintString` "Tactician Ready"))

(event `self.OnUnitSelection`
  (bind _ashud (cast `/Gamekit/HUD/HUD` (`self.GetHUD`)))
  (bind _returnvalue (`self.GetSelectedUnit`))
  (`/Gamekit/HUD/TestWidget.SetCharacterPreview` (`/Gamekit/HUD/HUD.MainWidget` _ashud) _returnvalue)
  (bind (_returnvalue_x _returnvalue_y _returnvalue_z) (`KismetMathLibrary.BreakVector` (`SceneComponent.K2_GetComponentLocation` (`Character.Mesh` _returnvalue))))
  (`KismetMaterialLibrary.SetVectorParameterValue` "/Gamekit/Tiles/TileMatParameters.TileMatParameters" "Unit Position" (make `LinearColor` _returnvalue_x _returnvalue_y _returnvalue_z 1.0))
  (`KismetMaterialLibrary.SetScalarParameterValue` "/Gamekit/Tiles/TileMatParameters.TileMatParameters" "Unit Range" 5.0)
  (`KismetMaterialLibrary.SetScalarParameterValue` "/Gamekit/Tiles/TileMatParameters.TileMatParameters" "Show Range" 1.0))

(event `self.OnUnitUnselect`
  (`/Gamekit/HUD/TestWidget.Remove Preview` (`/Gamekit/HUD/HUD.MainWidget` (stale `self.OnUnitSelection` _ashud)))
  (`KismetMaterialLibrary.SetScalarParameterValue` "/Gamekit/Tiles/TileMatParameters.TileMatParameters" "Show Range"))

(fn `UserConstructionScript`)